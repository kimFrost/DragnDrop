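; AllocationSlot is a Blueprint object that holds a single Allocatable.
; Allocate accepts a valid item only while empty, unallocating it first, then sets the two-way reference between slot and item.
; Unallocate clears that link only for the item currently held.
; Both notify slot and item of the change; AllowedID and AllowedClass filter nodes exist but are unused, so neither restricts allocation.
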(fn Allocate
  (params (Allocatable :type Allocatable%20Object%20Reference))
  (bind _self self)
  (Utilities|IsValid Allocatable
    (:Is%20Valid
      (if (not (Variables|Default|GetHasAllocation))
        (Default|Unallocate Allocatable)
        (bind _output_get (Variables|Default|SetAllocation Allocatable))
        (Variables|Default|SetHasAllocation true)
        (Variables|/Game/Allocatable/Blueprint/Objects/Allocatable.Allocatable_C|SetAllocatedTo _output_get self)
        (Default|CallOnAllocation _self _self)
        (Default|CallOnAllocated (Variables|Default|GetAllocation) (Variables|Default|GetAllocation))))))

(fn Unallocate
  (params (Allocatable :type Allocatable%20Object%20Reference))
  (bind _self self)
  (Utilities|IsValid Allocatable
    (:Is%20Valid
      (if (== Allocatable (Variables|Default|GetAllocation))
        (Variables|/Game/Allocatable/Blueprint/Objects/Allocatable.Allocatable_C|SetAllocatedTo (Variables|Default|GetAllocation) 0)
        (Default|CallOnUnallocated (Variables|Default|GetAllocation) (Variables|Default|GetAllocation))
        (Variables|Default|SetAllocation 0)
        (Variables|Default|SetHasAllocation false)
        (Default|CallOnUnallocation _self _self)))))