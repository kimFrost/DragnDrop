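; Socket object that holds a capped list of Allocatables whose ID matches its allowed ID.
; Allocate first detaches the item from its previous allocation, then links and binds it; Unallocate releases one item, or iterates over all when given an invalid reference.
; It relays items' activation events and broadcasts allocation changes.
; Average quality is recomputed on changes, dividing by maximum capacity so empty slots lower it.
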(event Custom|RemoveBindings
  (params (Allocation :type Allocatable%20Object%20Reference))
  (Utilities|IsValid Allocation
    (:Is%20Valid
      (EventDispatchers|UnbindEventfromOnActivated Allocation (delegate Custom|CustomEvent_0))
      (EventDispatchers|UnbindEventfromOnDeactivated Allocation (delegate Custom|CustomEvent_1))
      (EventDispatchers|UnbindEventfromOnQualityUpdate Allocation (delegate Custom|CustomEvent_2)))))

(event Custom|CustomEvent_0
  (params (Allocatable :type Allocatable%20Object%20Reference))
  (Default|CallOnActivated self))

(event Custom|CustomEvent_1
  (params (Allocatable :type Allocatable%20Object%20Reference))
  (Default|CallOnDeactivated self))

(event Custom|AddBindings
  (params (Allocation :type Allocatable%20Object%20Reference))
  (Utilities|IsValid Allocation
    (:Is%20Valid
      (EventDispatchers|BindEventtoOnActivated Allocation (delegate Custom|CustomEvent_0))
      (EventDispatchers|BindEventtoOnDeactivated Allocation (delegate Custom|CustomEvent_1))
      (EventDispatchers|BindEventtoOnQualityUpdate Allocation (delegate Custom|CustomEvent_2)))))

(event Custom|CustomEvent_2
  (params (Quality :type Float%20%28single-precision%29))
  (CallFunction|UpdateAvgValues))

(fn Allocate
  (params (Allocatable :type Allocatable%20Object%20Reference))
  (bind _self self)
  (Utilities|FlowControl|Sequence
    (:then_0
      (Utilities|IsValid Allocatable
        (:Is%20Valid
          (if (not (Variables|Default|GetIsFull))
            (if (Utilities|Enum|Equal(Enum) (Variables|Default|GetAllowedID) (Variables|/Game/Allocatable/Blueprint/Objects/Allocatable.Allocatable_C|GetID Allocatable))
              (Default|Unallocate Allocatable)
              (bind _returnvalue (Utilities|Array|Add (Variables|Default|GetAllocations) Allocatable))
              (Variables|Default|SetIsFull (== (- _returnvalue 1) (Variables|Default|GetMaxAllocated)))
              (Variables|/Game/Allocatable/Blueprint/Objects/Allocatable.Allocatable_C|SetAllocatedTo Allocatable self)
              (CallFunction|AddBindings Allocatable)
              (CallFunction|UpdateAvgValues)
              (Default|CallOnAllocation _self _self (Variables|Default|GetIsFull))
              (Default|CallOnAllocated Allocatable Allocatable)
              (return true))))))
    (:then_1
      (return false))))

(fn Unallocate
  (params (Allocatable :type Allocatable%20Object%20Reference))
  (bind _self self)
  (bind _allocations (Variables|Default|GetAllocations))
  (Utilities|IsValid Allocatable
    (:Is%20Valid
      (if (Utilities|Array|ContainsItem _allocations Allocatable)
        (CallFunction|RemoveBindings Allocatable)
        (Variables|/Game/Allocatable/Blueprint/Objects/Allocatable.Allocatable_C|SetAllocatedTo Allocatable 0)
        (Default|CallOnUnallocated Allocatable Allocatable)
        (Utilities|Array|RemoveItem (Variables|Default|GetAllocations) Allocatable)
        (Variables|Default|SetIsFull false)
        (CallFunction|UpdateAvgValues)
        (Default|CallOnUnallocation _self _self)))
    (:Is%20Not%20Valid
      (for _array_element _allocations
        (CallFunction|Unallocate _array_element)))))

(fn UpdateAvgValues
  (Variables|Default|SetAvgQuantity 0.0)
  (for _array_element (Variables|Default|GetAllocations)
    (Utilities|IsValid _array_element
      (:Is%20Valid
        (Variables|Default|SetAvgQuantity (+ (Variables|Default|GetAvgQuantity) (Variables|/Game/Allocatable/Blueprint/Objects/Allocatable.Allocatable_C|GetQuality _array_element))))))
  (bind _output_get (Variables|Default|SetAvgQuantity (/ (Variables|Default|GetAvgQuantity) (Math|Conversions|ToFloat(Integer) (Variables|Default|GetMaxAllocated)))))
  (Default|CallOnQualityUpdate _output_get))