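; Allocatable Blueprint object that can be allocated to a slot and switched between active and inactive states.
; Allocate proceeds only for a valid slot when the object is not already allocated, and Unallocate delegates release to the owner it is allocated to.
; Activate and Deactivate act only on a change of state, updating the active flag and broadcasting the matching event with itself as payload.
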(fn Allocate
  (params (Slot :type Allocation%20Slot%20Object%20Reference))
  (Utilities|IsValid Slot
    (:Is%20Valid
      (if (not (Variables|Default|GetIsAllocated))
        (CallFunction|Allocate Slot)))))

(fn Unallocate
  (bind _allocatedto (Variables|Default|GetAllocatedTo))
  (Utilities|IsValid _allocatedto
    (:Is%20Valid
      (Default|Unallocate _allocatedto self))))

(fn Activate
  (if (not (Variables|Default|GetIsActive))
    (Variables|Default|SetIsActive true)
    (Default|CallOnActivated self)))

(fn Deactivate
  (if (Variables|Default|GetIsActive)
    (Variables|Default|SetIsActive false)
    (Default|CallOnDeactivated self)))