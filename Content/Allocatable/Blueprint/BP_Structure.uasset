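; BP_Structure is a production building or hex tile that turns allocated inputs, including workers, into allocatable outputs.
; BeginPlay creates input slots and outputs; slot events trigger UpdateProduction, which toggles outputs on input readiness.
; Output quality multiplies average resource quality by average worker quality, counting empty slots as zero.
; Selection draws the range circle and shows the widget, plus matching supplier and consumer widgets on structures overlapping its range sphere.
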(event Custom|CustomEvent_0
  (params (Slot :type Allocation%20Slot%20Object%20Reference))
  (CallFunction|UpdateProduction))

(event Custom|CustomEvent_2
  (params (Slot :type Allocation%20Slot%20Object%20Reference))
  (CallFunction|UpdateProduction))

(event Custom|CustomEvent_1
  (params (Slot :type Allocation%20Slot%20Object%20Reference))
  (CallFunction|UpdateProduction))

(event Custom|CustomEvent_3
  (params (Slot :type Allocation%20Slot%20Object%20Reference))
  (CallFunction|UpdateProduction))

(event EventBeginPlay
  (bind _self self)
  (bind _self_2 self)
  (Utilities|FlowControl|Sequence
    (:then_0
      (for _array_element (Variables|Default|GetInput)
        (bind _returnvalue (Game|ConstructObjectfromClass "/Game/Allocatable/Blueprint/Objects/AllocationSlot.AllocationSlot_C" _self_2 0 "/Game/Allocatable/Blueprint/Objects/Allocatable.Allocatable_C" _array_element _self_2))
        (Utilities|Array|Add (Variables|Default|GetInputSlots) _returnvalue)
        (EventDispatchers|BindEventtoOnAllocation _returnvalue (delegate Custom|CustomEvent_0))
        (EventDispatchers|BindEventtoOnUnallocation _returnvalue (delegate Custom|CustomEvent_1))
        (EventDispatchers|BindEventtoOnActivated _returnvalue (delegate Custom|CustomEvent_2))
        (EventDispatchers|BindEventtoOnDeactivated _returnvalue (delegate Custom|CustomEvent_3))))
    (:then_1
      (for _array_element_2 (Variables|Default|GetOutput)
        (bind _returnvalue_2 (Game|ConstructObjectfromClass "/Game/Allocatable/Blueprint/Objects/Allocatable.Allocatable_C" _self _array_element_2 _self))
        (Default|SetQuality _returnvalue_2 (Variables|Default|GetQualityOverride))
        (Utilities|Array|Add (Variables|Default|GetOutputProduction) _returnvalue_2)))
    (:then_2
      (bind _returnvalue_3 (AddComponent|AddWidgetComponent false))
      (bind _output_get (Variables|Default|SetStructureWidgetComponent _returnvalue_3))
      (bind _aswidget_structure (Utilities|Casting|CastToWidget_Structure (UserInterface|GetUserWidgetObject _output_get)))
      (Variables|/Game/Allocatable/Blueprint/UI/Widget_Structure.Widget_Structure_C|SetStructure _aswidget_structure self))
    (:then_3
      (CallFunction|UpdateProduction)
      (CallFunction|Deselect))))

(event EventTick
  (params (DeltaSeconds :type Float%20%28single-precision%29))
  (if (Variables|Default|GetIsSelected)
    (Rendering|Debug|DrawDebugCircle (Transformation|GetActorLocation) (Variables|Default|GetMaxDistanceToStructure) 64 "(R=0.159303,G=1.000000,B=0.000000,A=1.000000)" 0.0 1e+01 "0.000000,1.000000,0.000000" "1.000000,0.000000,0.000000")))

(fn ConstructionScript
  (Components|Sphere|SetSphereRadius (Variables|Default|GetSphere) (Variables|Default|GetMaxDistanceToStructure) true)
  (Rendering|Components|TextRender|SetText (Variables|Default|GetTitleText) (Utilities|Text|ToText(String) (Variables|Default|GetTitle)))
  (if (Variables|Default|GetIsTile)
    (Components|StaticMesh|SetStaticMesh (Variables|Default|GetStaticMesh) "/Game/Allocatable/Meshes/SM_Hex.SM_Hex")))

(fn UpdateProduction
  (CallFunction|UpdateQuality)
  (Utilities|FlowControl|Sequence
    (:then_0
      (Variables|Default|SetHasAllInputsAllocation true)
      (bind _array_element (Utilities|Array|ForEachLoopwithBreak (Variables|Default|GetInputSlots) :!label _label)
        (:LoopBody
          (Utilities|IsValid _array_element
            (:Is%20Valid
              (if (Variables|/Game/Allocatable/Blueprint/Objects/AllocationSlot.AllocationSlot_C|GetHasAllocation _array_element)
                (Utilities|IsValid (Variables|/Game/Allocatable/Blueprint/Objects/AllocationSlot.AllocationSlot_C|GetAllocation _array_element)
                  (:Is%20Valid
                    (if (not (Variables|/Game/Allocatable/Blueprint/Objects/Allocatable.Allocatable_C|GetIsActive (Variables|/Game/Allocatable/Blueprint/Objects/AllocationSlot.AllocationSlot_C|GetAllocation _array_element)))
                      (Variables|Default|SetHasAllInputsAllocation false :!label _label_2)
                      (goto _label Break)))
                  (:Is%20Not%20Valid
                    (goto _label_2)))
                (else
                  (goto _label_2))))))))
    (:then_1
      (for _array_element_2 (Variables|Default|GetOutputProduction)
        (Utilities|IsValid _array_element_2
          (:Is%20Valid
            (if (Variables|Default|GetHasAllInputsAllocation)
              (Default|Activate _array_element_2)
              (else
                (Default|Deactivate _array_element_2)))))))
    (:then_2
      (Default|CallOnProductionUpdated))))

(fn Select
  (Variables|Default|SetIsSelected true)
  (CallFunction|ShowUI true true)
  (for _array_element (Collision|GetOverlappingActors (Variables|Default|GetSphere) "BP_Structure_C" :!class /Script/Engine.PrimitiveComponent)
    (bind _asbp_structure (Utilities|Casting|CastToBP_Structure _array_element))
    (Utilities|IsValid _asbp_structure
      (:Is%20Valid
        (Utilities|FlowControl|Sequence
          (:then_0
            (for _array_element_2 (Variables|Default|GetInput)
              (if (Utilities|Array|ContainsItem (Variables|BP_Structure_C|GetOutput _asbp_structure) _array_element_2)
                (CallFunction|ShowUI _asbp_structure false true))))
          (:then_1
            (for _array_element_3 (Variables|Default|GetOutput)
              (if (Utilities|Array|ContainsItem (Variables|BP_Structure_C|GetInput _asbp_structure) _array_element_3)
                (CallFunction|ShowUI _asbp_structure true false)))))))))

(fn Deselect
  (Variables|Default|SetIsSelected false)
  (CallFunction|HideUI))

(fn ShowUI
  (params (ShowInput :type Boolean) (ShowOutput :type Boolean))
  (Rendering|SetVisibility (Variables|Default|GetStructureWidgetComponent) true false)
  (bind _aswidget_structure (Utilities|Casting|CastToWidget_Structure (UserInterface|GetUserWidgetObject (Variables|Default|GetStructureWidgetComponent))))
  (Default|HideInputs _aswidget_structure)
  (Default|HideOutputs _aswidget_structure)
  (Utilities|FlowControl|Sequence
    (:then_0
      (if ShowInput
        (Default|ShowInputs _aswidget_structure)))
    (:then_1
      (if ShowOutput
        (Default|ShowOutputs _aswidget_structure)))))

(fn HideUI
  (Rendering|SetVisibility (Variables|Default|GetStructureWidgetComponent) false false))

(fn UpdateQuality
  (Utilities|FlowControl|Sequence
    (:then_0
      (Variables|Default|SetAvgResourceInputQuality 0.0)
      (Variables|Default|SetAvgWorkerInputQuality 0.0)
      (Variables|Default|SetNumOfInputWorkers 0)
      (Variables|Default|SetNumOfInputResources 0)
      (for _array_element (Variables|Default|GetInputSlots)
        (Utilities|IsValid _array_element
          (:Is%20Valid
            (Utilities|IsValid (Variables|/Game/Allocatable/Blueprint/Objects/AllocationSlot.AllocationSlot_C|GetAllocation _array_element)
              (:Is%20Valid
                (if (Variables|/Game/Allocatable/Blueprint/Objects/AllocationSlot.AllocationSlot_C|GetHasAllocation _array_element)
                  (if (Utilities|Enum|Equal(Enum) (Variables|/Game/Allocatable/Blueprint/Objects/Allocatable.Allocatable_C|GetID (Variables|/Game/Allocatable/Blueprint/Objects/AllocationSlot.AllocationSlot_C|GetAllocation _array_element)) "Worker")
                    (Variables|Default|SetAvgWorkerInputQuality (+ (Variables|Default|GetAvgWorkerInputQuality) (Variables|/Game/Allocatable/Blueprint/Objects/Allocatable.Allocatable_C|GetQuality (Variables|/Game/Allocatable/Blueprint/Objects/AllocationSlot.AllocationSlot_C|GetAllocation _array_element))))
                    (Math|Integer|IncrementInt (Variables|Default|GetNumOfInputWorkers))
                    (else
                      (Variables|Default|SetAvgResourceInputQuality (+ (Variables|Default|GetAvgResourceInputQuality) (Variables|/Game/Allocatable/Blueprint/Objects/Allocatable.Allocatable_C|GetQuality (Variables|/Game/Allocatable/Blueprint/Objects/AllocationSlot.AllocationSlot_C|GetAllocation _array_element))))
                      (Math|Integer|IncrementInt (Variables|Default|GetNumOfInputResources))))))
              (:Is%20Not%20Valid
                (if (Utilities|Enum|Equal(Enum) (Variables|/Game/Allocatable/Blueprint/Objects/AllocationSlot.AllocationSlot_C|GetAllowedID _array_element) "Worker")
                  (Math|Integer|IncrementInt (Variables|Default|GetNumOfInputWorkers))
                  (else
                    (Math|Integer|IncrementInt (Variables|Default|GetNumOfInputResources))))))))))
    (:then_1
      (Utilities|FlowControl|Sequence
        (:then_0
          (Variables|Default|SetAvgResourceInputQuality (/ (Variables|Default|GetAvgResourceInputQuality) (Math|Conversions|ToFloat(Integer) (Variables|Default|GetNumOfInputResources)))))
        (:then_1
          (Variables|Default|SetAvgWorkerInputQuality (/ (Variables|Default|GetAvgWorkerInputQuality) (Math|Conversions|ToFloat(Integer) (Variables|Default|GetNumOfInputWorkers)))))
        (:then_2
          (Variables|Default|SetOutputQuality (* (Variables|Default|GetAvgResourceInputQuality) (Variables|Default|GetAvgWorkerInputQuality))))))
    (:then_2
      (if (> (Utilities|Array|Length (Variables|Default|GetInputSlots)) 0)
        (for _array_element_2 (Variables|Default|GetOutputProduction)
          (Utilities|IsValid _array_element_2
            (:Is%20Valid
              (Default|SetQuality _array_element_2 (Variables|Default|GetOutputQuality)))))))))

(fn DestroyStructure
  (for _array_element (Variables|Default|GetInputSlots)
    (Utilities|IsValid _array_element
      (:Is%20Valid
        (Default|Unallocate _array_element (Variables|/Game/Allocatable/Blueprint/Objects/AllocationSlot.AllocationSlot_C|GetAllocation _array_element)))))
  (for _array_element_2 (Variables|Default|GetOutputProduction)
    (Utilities|IsValid _array_element_2
      (:Is%20Valid
        (Default|Unallocate _array_element_2))))
  (Actor|DestroyActor))