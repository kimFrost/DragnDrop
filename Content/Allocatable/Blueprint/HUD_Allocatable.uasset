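; HUD that shows the allocation UI and draws wires between connected allocation slots.
; BeginPlay adds the AllocateableHUD widget to the viewport.
; Each DrawHUD gathers all InputSlot widgets and, for visible connected pairs, draws a curve from output to input screen position as short line segments via GetCurveBetweenPoints.
; Disconnected leftovers of straight and jittered line drawing never run.
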(event EventBeginPlay
  (bind _returnvalue (UserInterface|CreateWidget "/Game/Allocatable/Blueprint/UI/Widget_Allocateable-HUD.Widget_Allocateable-HUD_C"))
  (UserInterface|Viewport|AddtoViewport _returnvalue 0))

(event Collision|EventActorBeginOverlap
  (params (OtherActor :type Actor%20Object%20Reference)))

(event EventTick
  (params (DeltaSeconds :type Float%20%28single-precision%29)))

(event EventDrawHUD
  (params (SizeX :type Integer) (SizeY :type Integer))
  (bind _foundwidgets (Widget|GetAllWidgetsOfClass "/Game/Allocatable/Blueprint/UI/Widget_InputSlot.Widget_InputSlot_C" false))
  (for _array_element _foundwidgets
    (Utilities|IsValid _array_element
      (:Is%20Valid
        (Utilities|IsValid (Variables|/Game/Allocatable/Blueprint/UI/Widget_InputSlot.Widget_InputSlot_C|GetAllocationSlot _array_element)
          (:Is%20Valid
            (for _array_element_2 (Variables|/Game/Allocatable/Blueprint/UI/Widget_InputSlot.Widget_InputSlot_C|GetConnectedTo _array_element)
              (Utilities|IsValid _array_element_2
                (:Is%20Valid
                  (if (and (Widget|IsVisible _array_element) (Widget|IsVisible _array_element_2))
                    (bind _returnvalue (Class|AllocatableHelpers|GetCurveBetweenPoints (Math|Conversions|ToVector(Vector2D) (Variables|/Game/Allocatable/Blueprint/UI/Widget_OutputSlot.Widget_OutputSlot_C|GetOutputScreenPosition _array_element_2)) (Math|Conversions|ToVector(Vector2D) (Variables|/Game/Allocatable/Blueprint/UI/Widget_InputSlot.Widget_InputSlot_C|GetInputScreenPosition _array_element))))
                    (for (_array_element_3 _array_index) _returnvalue
                      (if (!= _array_index (- (Utilities|Array|Length _returnvalue) 1))
                        (Class|HUD|DrawLine (.X (Math|Vector2D|BreakVector2D (Math|Conversions|ToVector2D(Vector) _array_element_3))) (.Y (Math|Vector2D|BreakVector2D (Math|Conversions|ToVector2D(Vector) _array_element_3))) (.X (Math|Vector2D|BreakVector2D (Math|Conversions|ToVector2D(Vector) (Utilities|Array|Get(acopy) _returnvalue (+ _array_index 1))))) (.Y (Math|Vector2D|BreakVector2D (Math|Conversions|ToVector2D(Vector) (Utilities|Array|Get(acopy) _returnvalue (+ _array_index 1))))) "(R=0.420053,G=0.000000,B=1.000000,A=1.000000)" 2.0)))))))))))))

(fn ConstructionScript)