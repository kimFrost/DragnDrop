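; Construction site that stands in for a structure being built, then spawns the finished BP_Structure and removes itself.
; On BeginPlay it rewrites its row data so the construction cost becomes its inputs, with no outputs.
; Tick drains the remaining build time at a rate set by OutputQuality and refreshes progress and time-left texts.
; At zero it looks up WhatToBuild in DATA_Structures for the spawn; the production-updated handler is an empty stub.
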(event Custom|OnProductionUpdated_Event
  (if (Variables|Default|GetHasAllInputsAllocation)
    _))

(event EventTick
  (params (DeltaSeconds :type Float%20%28single-precision%29))
  (|CallParentFunction DeltaSeconds)
  (if (> (Variables|Default|GetOutputQuality) 0.0)
    (bind _output_get (Variables|Default|SetBuildTimeLeft (- (Variables|Default|GetBuildTimeLeft) (* (Variables|Default|GetOutputQuality) DeltaSeconds))))
    (if (<= _output_get 0.0)
      (Utilities|FlowControl|Sequence
        (:then_0
          (bind _returnvalue (Utilities|GetDataTableRow "/Game/Allocatable/Blueprint/Structs/DATA_Structures.DATA_Structures" (Utilities|String|StringToName (Variables|Default|GetWhatToBuild)))
            (:then
              (Game|SpawnActorfromClass "/Game/Allocatable/Blueprint/BP_Structure.BP_Structure_C" (Transformation|GetActorTransform) "Undefined" 0 (.ID (Utilities|Struct|BreakST_Structure _returnvalue)) 1.0 false _returnvalue false 0))))
        (:then_1
          (CallFunction|DestroyStructure)))
      (else
        (Utilities|FlowControl|Sequence :!label _label
          (:then_1
            (Rendering|Components|TextRender|SetText (Variables|Default|GetPercentCompletedText) (Utilities|Text|ToText(String) (Utilities|String|BuildString(Float) "" "" (- 1.0 (Variables|Default|GetBuildPercentLeft)) "%"))))
          (:then_2
            (Rendering|Components|TextRender|SetText (Variables|Default|GetBuildTimeLeftText) (Utilities|Text|ToText(String) (Utilities|String|SelectString (Utilities|String|BuildString(Float) "" "" (/ (Variables|Default|GetBuildTimeLeft) (Variables|Default|GetOutputQuality)) "s") "-s" (> (/ (Variables|Default|GetBuildTimeLeft) (Variables|Default|GetOutputQuality)) 0.0))))))))
    (else
      (goto _label))))

(event EventBeginPlay
  (bind _buildtimeleft (Variables|Default|GetBuildTimeLeft))
  (bind _outputquality (Variables|Default|GetOutputQuality))
  (bind _returnvalue (/ _buildtimeleft _outputquality))
  (Variables|Default|SetRowData (Utilities|Struct|MakeST_Structure (.ID (Utilities|Struct|BreakST_Structure (Variables|Default|GetRowData))) (.ConstructionCost (Utilities|Struct|BreakST_Structure (Variables|Default|GetRowData))) (Utilities|Array|MakeArray) (.ConstructionCost (Utilities|Struct|BreakST_Structure (Variables|Default|GetRowData))) (.ConstructionTime (Utilities|Struct|BreakST_Structure (Variables|Default|GetRowData)))))
  (|CallParentFunction)
  (EventDispatchers|BindEventtoOnProductionUpdated (delegate Custom|OnProductionUpdated_Event))
  (if (<= (stale EventTick _output_get) 0.0)
    (Utilities|FlowControl|Sequence
      (:then_0
        (bind _returnvalue_2 (Utilities|GetDataTableRow "/Game/Allocatable/Blueprint/Structs/DATA_Structures.DATA_Structures" (Utilities|String|StringToName (Variables|Default|GetWhatToBuild)))
          (:then
            (Game|SpawnActorfromClass "/Game/Allocatable/Blueprint/BP_Structure.BP_Structure_C" (Transformation|GetActorTransform) "Undefined" 0 (.ID (Utilities|Struct|BreakST_Structure _returnvalue_2)) 1.0 false _returnvalue_2 false 0))))
      (:then_1
        (CallFunction|DestroyStructure)))
    (else
      (Utilities|FlowControl|Sequence
        (:then_1
          (Rendering|Components|TextRender|SetText (Variables|Default|GetPercentCompletedText) (Utilities|Text|ToText(String) (Utilities|String|BuildString(Float) "" "" (- 1.0 (Variables|Default|GetBuildPercentLeft)) "%"))))
        (:then_2
          (Rendering|Components|TextRender|SetText (Variables|Default|GetBuildTimeLeftText) (Utilities|Text|ToText(String) (Utilities|String|SelectString (Utilities|String|BuildString(Float) "" "" _returnvalue "s") "-s" (> _returnvalue 0.0)))))))))

(fn ConstructionScript
  (|CallParentFunction))