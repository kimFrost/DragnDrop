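; Player controller for a building game, handling structure placement and selection through cursor visibility traces.
; Number keys choose a building type and immediately spawn a BP_ConstructionSite at the cursor with its DATA_Structures row, unless a BP_Structure is under it.
; Left-click on a structure makes it the sole selection; right-click deselects all structures without clearing SelectedStructures.
; Tick draws a debug circle at the cursor hit point.
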(event EventBeginPlay)

(event EventTick
  (params (DeltaSeconds :type Float%20%28single-precision%29))
  (bind (_hitresult _returnvalue) (Game|Player|GetHitResultUnderCursorbyChannel "TraceTypeQuery1" true))
  (if _returnvalue
    (Rendering|Debug|DrawDebugCircle (.Location (Collision|BreakHitResult _hitresult)) 1e+03 64 "(R=1.000000,G=1.000000,B=1.000000,A=1.000000)" 0.0 1e+01 "0.000000,1.000000,0.000000" "1.000000,0.000000,0.000000")))

(event Input|MouseEvents|LeftMouseButton
  (params (Key :type Key%20Structure))
  (bind (_hitresult _returnvalue) (Game|Player|GetHitResultUnderCursorbyChannel "TraceTypeQuery1" true))
  (:Released
    (if _returnvalue
      (bind _asbp_structure (Utilities|Casting|CastToBP_Structure (.HitActor (Collision|BreakHitResult _hitresult))))
      (bind _outactors (Actor|GetAllActorsOfClass "/Game/Allocatable/Blueprint/BP_Structure.BP_Structure_C"))
      (for _array_element _outactors
        (Utilities|IsValid _array_element
          (:Is%20Valid
            (Default|Deselect _array_element))))
      (Utilities|Array|Clear (Variables|Default|GetSelectedStructures))
      (Default|Select _asbp_structure)
      (Utilities|Array|Add (Variables|Default|GetSelectedStructures) _asbp_structure))))

(event Input|MouseEvents|RightMouseButton
  (params (Key :type Key%20Structure))
  (:Released
    (bind _outactors (Actor|GetAllActorsOfClass "/Game/Allocatable/Blueprint/BP_Structure.BP_Structure_C"))
    (for _array_element _outactors
      (Utilities|IsValid _array_element
        (:Is%20Valid
          (Default|Deselect _array_element))))))

(event Input|KeyboardEvents|1
  (params (Key :type Key%20Structure))
  (bind (_hitresult _returnvalue) (Game|Player|GetHitResultUnderCursorbyChannel "TraceTypeQuery1" true))
  (bind (_bblockinghit _binitialoverlap _time _location _impactpoint _normal _impactnormal _physmat _hitactor) (Collision|BreakHitResult _hitresult))
  (:Pressed
    (Variables|Default|SetWhatToBuild "House")
    (if _returnvalue
      (Utilities|Casting|CastToBP_Structure _hitactor
        (:CastFailed
          (bind _returnvalue_2 (Utilities|GetDataTableRow "/Game/Allocatable/Blueprint/Structs/DATA_Structures.DATA_Structures" (Utilities|String|StringToName (Variables|Default|GetWhatToBuild)))
            (:then
              (Game|SpawnActorfromClass "/Game/Allocatable/Blueprint/BP_ConstructionSite.BP_ConstructionSite_C" (Math|Conversions|ToTransform(Vector) _location) "Undefined" 0 (Variables|Default|GetWhatToBuild) (.ConstructionTime (Utilities|Struct|BreakST_Structure _returnvalue_2)) (Variables|Default|GetWhatToBuild) 1.0 false _returnvalue_2 false 0))))))))

(event Input|KeyboardEvents|2
  (params (Key :type Key%20Structure))
  (bind (_hitresult _returnvalue) (Game|Player|GetHitResultUnderCursorbyChannel "TraceTypeQuery1" true))
  (bind (_bblockinghit _binitialoverlap _time _location _impactpoint _normal _impactnormal _physmat _hitactor) (Collision|BreakHitResult _hitresult))
  (:Pressed
    (Variables|Default|SetWhatToBuild "Woodcutter")
    (if _returnvalue
      (Utilities|Casting|CastToBP_Structure _hitactor
        (:CastFailed
          (bind _returnvalue_2 (Utilities|GetDataTableRow "/Game/Allocatable/Blueprint/Structs/DATA_Structures.DATA_Structures" (Utilities|String|StringToName (Variables|Default|GetWhatToBuild)))
            (:then
              (Game|SpawnActorfromClass "/Game/Allocatable/Blueprint/BP_ConstructionSite.BP_ConstructionSite_C" (Math|Conversions|ToTransform(Vector) _location) "Undefined" 0 (Variables|Default|GetWhatToBuild) (.ConstructionTime (Utilities|Struct|BreakST_Structure _returnvalue_2)) (Variables|Default|GetWhatToBuild) 1.0 false _returnvalue_2 false 0))))))))

(event Input|KeyboardEvents|3
  (params (Key :type Key%20Structure))
  (bind (_hitresult _returnvalue) (Game|Player|GetHitResultUnderCursorbyChannel "TraceTypeQuery1" true))
  (bind (_bblockinghit _binitialoverlap _time _location _impactpoint _normal _impactnormal _physmat _hitactor) (Collision|BreakHitResult _hitresult))
  (:Pressed
    (Variables|Default|SetWhatToBuild "Lumbermill")
    (if _returnvalue
      (Utilities|Casting|CastToBP_Structure _hitactor
        (:CastFailed
          (bind _returnvalue_2 (Utilities|GetDataTableRow "/Game/Allocatable/Blueprint/Structs/DATA_Structures.DATA_Structures" (Utilities|String|StringToName (Variables|Default|GetWhatToBuild)))
            (:then
              (Game|SpawnActorfromClass "/Game/Allocatable/Blueprint/BP_ConstructionSite.BP_ConstructionSite_C" (Math|Conversions|ToTransform(Vector) _location) "Undefined" 0 (Variables|Default|GetWhatToBuild) (.ConstructionTime (Utilities|Struct|BreakST_Structure _returnvalue_2)) (Variables|Default|GetWhatToBuild) 1.0 false _returnvalue_2 false 0))))))))

(event Input|KeyboardEvents|4
  (params (Key :type Key%20Structure))
  (bind (_hitresult _returnvalue) (Game|Player|GetHitResultUnderCursorbyChannel "TraceTypeQuery1" true))
  (bind (_bblockinghit _binitialoverlap _time _location _impactpoint _normal _impactnormal _physmat _hitactor) (Collision|BreakHitResult _hitresult))
  (:Pressed
    (Variables|Default|SetWhatToBuild "Well")
    (if _returnvalue
      (Utilities|Casting|CastToBP_Structure _hitactor
        (:CastFailed
          (bind _returnvalue_2 (Utilities|GetDataTableRow "/Game/Allocatable/Blueprint/Structs/DATA_Structures.DATA_Structures" (Utilities|String|StringToName (Variables|Default|GetWhatToBuild)))
            (:then
              (Game|SpawnActorfromClass "/Game/Allocatable/Blueprint/BP_ConstructionSite.BP_ConstructionSite_C" (Math|Conversions|ToTransform(Vector) _location) "Undefined" 0 (Variables|Default|GetWhatToBuild) (.ConstructionTime (Utilities|Struct|BreakST_Structure _returnvalue_2)) (Variables|Default|GetWhatToBuild) 1.0 false _returnvalue_2 false 0))))))))

(event Input|KeyboardEvents|5
  (params (Key :type Key%20Structure))
  (bind (_hitresult _returnvalue) (Game|Player|GetHitResultUnderCursorbyChannel "TraceTypeQuery1" true))
  (bind (_bblockinghit _binitialoverlap _time _location _impactpoint _normal _impactnormal _physmat _hitactor) (Collision|BreakHitResult _hitresult))
  (:Pressed
    (Variables|Default|SetWhatToBuild "Fisherhut")
    (if _returnvalue
      (Utilities|Casting|CastToBP_Structure _hitactor
        (:CastFailed
          (bind _returnvalue_2 (Utilities|GetDataTableRow "/Game/Allocatable/Blueprint/Structs/DATA_Structures.DATA_Structures" (Utilities|String|StringToName (Variables|Default|GetWhatToBuild)))
            (:then
              (Game|SpawnActorfromClass "/Game/Allocatable/Blueprint/BP_ConstructionSite.BP_ConstructionSite_C" (Math|Conversions|ToTransform(Vector) _location) "Undefined" 0 (Variables|Default|GetWhatToBuild) (.ConstructionTime (Utilities|Struct|BreakST_Structure _returnvalue_2)) (Variables|Default|GetWhatToBuild) 1.0 false _returnvalue_2 false 0))))))))

(fn ConstructionScript)